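; Survivor player character that randomizes its skeletal mesh, plays breathing audio and leaves trail decals.
; BeginPlay calls server and multicast mesh events, with the random pick made inside the multicast, and plays 2D breathing.
; A looping timer feeds the distance to the first killer, in meters, into an audio parameter.
; HandleFootprints traces downward to spawn fading scratchmark decals, plus DoOnce-throttled blood decals when injured.
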(event `Server_AssignRandomMesh`
  (`self.Multi_AssignRandomMesh`))

(event `Multi_AssignRandomMesh`
  (`SkeletalMeshComponent.SetSkeletalMeshAsset` (`self.Mesh`) (`KismetArrayLibrary.Array_Random` (`self.RandomMesh`))))

(event `self.ReceiveBeginPlay`
  (`self.Server_AssignRandomMesh`)
  (`self.Multi_AssignRandomMesh`)
  (`GameplayStatics.PlaySound2D` "/Game/Audio/Cues/Characters/Survivor/SFX_GirlBreathing.SFX_GirlBreathing" 1.0 1.0 0.0 null null)
  (`self.KillerDistance`)
  (`KismetSystemLibrary.K2_SetTimerDelegate` (delegate `KillerDistance`) 1.0 true))

(event `KillerDistance`
  (bind _outactors (`GameplayStatics.GetAllActorsOfClass` "/Game/Blueprints/Player/Characters/BP_KillerCharacter.BP_KillerCharacter_C"))
  (bind _output (`|GetArrayItem` _outactors))
  (`/Engine/EditorBlueprintResources/StandardMacros.IsValid` _output
    (:`Is Valid`
      (message `AudioParameterControllerInterface.SetFloatParameter` (`self.KillerDistanceAudio`) "KillerDistance" (/ (`self.GetDistanceTo` _output self) 100.0)))))

(event `HandleFootprints`
  (params (IsInjured :type Boolean))
  (bind _returnvalue (`self.K2_GetActorLocation`))
  (bind _outhit (`KismetSystemLibrary.LineTraceSingle` _returnvalue (+ _returnvalue (* (`self.GetActorUpVector`) -200.0)) "TraceTypeQuery1"))
  (bind (_bblockinghit _binitialoverlap _time _distance _location) (`GameplayStatics.BreakHitResult` _outhit))
  (bind _returnvalue_2 (`GameplayStatics.SpawnDecalAtLocation` "/Game/Assets/VFX/Decals/M_ScratchmarkDecal.M_ScratchmarkDecal" (5.0 200.0 200.0) _location))
  (`/Engine/EditorBlueprintResources/StandardMacros.IsValid` _returnvalue_2
    (:`Is Valid`
      (`DecalComponent.SetFadeIn` _returnvalue_2 0.0 1.0)
      (`DecalComponent.SetFadeOut` _returnvalue_2 9.0 1.0 false))
    (:`Is Not Valid`
      _))
  (if IsInjured
    (`/Engine/EditorBlueprintResources/StandardMacros.DoOnce` false :!label _label
      (:`Completed`
        (bind _returnvalue_3 (`GameplayStatics.SpawnDecalAtLocation` "/Game/Assets/VFX/Decals/M_BloodDecal.M_BloodDecal" (5.0 80.0 80.0) _location))
        (`/Engine/EditorBlueprintResources/StandardMacros.IsValid` _returnvalue_3
          (:`Is Valid`
            (`DecalComponent.SetFadeIn` _returnvalue_3 0.0 1.0)
            (`DecalComponent.SetFadeOut` _returnvalue_3 9.0 1.0 false)
            (`KismetSystemLibrary.Delay` 1.0)
            (goto _label :!via `Reset`)))))))

(fn `UserConstructionScript`)